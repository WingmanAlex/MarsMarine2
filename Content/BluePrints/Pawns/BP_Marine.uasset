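; BP_Marine is the player-controlled marine, with world-axis movement and twin-stick-style aiming by gamepad or mouse.
; Any key press records whether a gamepad is active, and Tick sets control yaw from the thumbstick angle or smoothed mouse-movement direction, each past a deadzone.
; Fire input toggles the rifle muzzle flash and firing sounds, with no shot or damage logic here.
; BeginPlay creates the player HUD with a reference to the marine.
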(event `self.ReceiveTick`
  (params (DeltaSeconds :type "Float (single-precision)"))
  ;[0.3438 0.3438 0.3438] Input
  ;;[1 1 1] Choses gamepad or mouse each tick
  (`self.Update Player Aim`))

(event `InputAxis|MoveForward`
  (params (AxisValue :type "Float (single-precision)"))
  ;[0.3438 0.3438 0.3438] Input
  ;;[1 1 1] Input set up foward/backward - left/right
  (`self.AddMovementInput` (1.0 0.0 0.0) AxisValue))

(event `InputAxis|MoveRight`
  (params (AxisValue :type "Float (single-precision)"))
  ;[0.3438 0.3438 0.3438] Input
  ;;[1 1 1] Input set up foward/backward - left/right
  (`self.AddMovementInput` (0.0 1.0 0.0) AxisValue))

(event `Key|AnyKey`
  (params (Key :type "Key Structure"))
  ;[0.3438 0.3438 0.3438] Input
  ;;[1 1 1] Checks if gamepad is active input
  (:`Pressed`
    (set `self.GamePad Active` (`KismetInputLibrary.Key_IsGamepadKey` Key))))

(event `InputAction|Fire Weapon`
  (params (Key :type "Key Structure"))
  ;[0.3438 0.3438 0.3438] Input
  ;;[1 1 1] Fire muzzle flash, audio
  (:`Pressed`
    (`self.Start Firing Weapon`))
  (:`Released`
    (`self.Stop Firing Weapon`)))

(event `self.ReceiveBeginPlay`
  ;[0.4509 1 0.394] HUD, Spawn, Marine ref,
  (bind _returnvalue (`|CreateWidget` "/Game/UI/W_PlayerHud.W_PlayerHUD_C" null self))
  (`UserWidget.AddToViewport` _returnvalue 0))

(fn `Get Mouse Aim Direction`
  (returns (ReturnValue :type "Rotator Structure"))
  (bind (_returnvalue_x _returnvalue_y) (`KismetMathLibrary.BreakVector2D` (`self.Get Mouse Velocity`)))
  ;[1 1 1] Mouse Directions
  (return (`KismetMathLibrary.RInterpTo` (`Controller.GetControlRotation` (`GameplayStatics.GetPlayerController` 0)) (`KismetMathLibrary.MakeRotator` 0.0 0.0 (`KismetMathLibrary.DegAtan2` _returnvalue_y _returnvalue_x)) (`GameplayStatics.GetWorldDeltaSeconds`) (`self.Mouse Smoothing Strength`))))

(fn `Get Mouse Velocity`
  (returns (ReturnValue :type "Vector2D Structure"))
  (bind (_deltax _deltay) (`PlayerController.GetInputMouseDelta` (`GameplayStatics.GetPlayerController` 0)))
  ;[1 1 1] Mouse Velocity
  (return (/ (`KismetMathLibrary.MakeVector2D` _deltax _deltay) (`GameplayStatics.GetWorldDeltaSeconds`))))

(fn `Get Thumbstick Aim Direction`
  (returns (ReturnValue :type "Rotator Structure"))
  ;[1 1 1] Converts values to degrees
  (return (`KismetMathLibrary.MakeRotator` 0.0 0.0 (`KismetMathLibrary.DegAtan2` (`self.GetInputAxisValue`) (`self.GetInputAxisValue`)))))

(fn `Is Mouse Above Deadzone`
  (returns (ReturnValue :type Boolean))
  ;[1 1 1] Is mouse in deadzone
  (return (> (`KismetMathLibrary.VSize2D` (`self.Get Mouse Velocity`)) (`self.Mouse Deadzone`))))

(fn `Is Thumbstick Above Deadzone`
  (returns (ReturnValue :type Boolean))
  ;[1 1 1] Is thumbstick input greater than thumbstick deadzone?
  (return (> (`KismetMathLibrary.VSize2D` (`KismetMathLibrary.MakeVector2D` (`self.GetInputAxisValue`) (`self.GetInputAxisValue`))) (`self.Thumbstick Deadzone`))))

(fn `Start Firing Weapon`
  ;[1 1 1] Activates Mussle Flash Particle, sound
  (`ActorComponent.Activate` (`self.P_AssaultRifle_MF`) false)
  (bind _returnvalue (`GameplayStatics.SpawnSound2D` "/Game/Sounds/Weapon_AssaultRifle/Stereo/RifleFire_Cue.RifleFire_Cue" 1.0 1.0 0.0 null))
  (set `self.Weapon Fire Sound` _returnvalue))

(fn `Stop Firing Weapon`
  ;[1 1 1] Deactivates Mussle flash & Sound
  (`ActorComponent.Deactivate` (`self.P_AssaultRifle_MF`))
  (`AudioComponent.Stop` (`self.Weapon Fire Sound`))
  (`GameplayStatics.SpawnSound2D` "/Game/Sounds/Weapon_AssaultRifle/Stereo/RifleFireEnd_Cue.RifleFireEnd_Cue" 1.0 1.0 0.0 null))

(fn `Update Mouse Aim`
  ;[1 1 1] Update mouse aim, velocity/delta, deadzone
  (if (`self.Is Mouse Above Deadzone`)
    (`Controller.SetControlRotation` (`GameplayStatics.GetPlayerController` 0) (`self.Get Mouse Aim Direction`))))

(fn `Update Player Aim`
  ;[1 1 1] Choses between input - gamepad/Mouse
  (if (`self.GamePad Active`)
    (`self.Update Thumbstick Aim`)
    (else
      (`self.Update Mouse Aim`))))

(fn `Update Thumbstick Aim`
  ;[1 1 1] Controller Rotation thumbstick + deadzone
  (if (`self.Is Thumbstick Above Deadzone`)
    (`Controller.SetControlRotation` (`GameplayStatics.GetPlayerController` 0) (`self.Get Thumbstick Aim Direction`))))

(fn `UserConstructionScript`)
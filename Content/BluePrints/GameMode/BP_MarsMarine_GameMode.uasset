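; Game mode for Mars Marine that starts an alien wave shortly after play begins.
; SetupNewWave increments the wave counter once and starts a looping timer, never cleared here, to trigger Spawn Wave every second.
; Each spawn places a BP_Alien at a random TargetPoint gathered from the level.
; The random index uses LastIndex as an exclusive maximum, so the last TargetPoint is never picked when several exist.
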(event `self.ReceiveBeginPlay`
  ;[1 1 1] Set up wave after 2 sec
  (`KismetSystemLibrary.Delay` 2.0)
  (`self.Setup New Wave`))

(event `Spawn Wave`
  (`self.Spawn Alien`))

(fn `Get Random Spawn Point`
  (returns (`Spawn Point` :type "Actor Object Reference"))
  ;[1 1 1] Get Random Target point in level
  (bind _outactors (`GameplayStatics.GetAllActorsOfClass` "/Script/Engine.TargetPoint"))
  (return (`|GetArrayItem` _outactors (`KismetMathLibrary.RandomInteger` (`KismetArrayLibrary.Array_LastIndex` _outactors)))))

(fn `Setup New Wave`
  ;[1 1 1] increase number to new wave
  (`/Engine/EditorBlueprintResources/StandardMacros.IncrementInt` (`self.Current Wave`)
    (:`  `
      ;[1 1 1] Spawn every second
      (`KismetSystemLibrary.K2_SetTimer` null "Spawn Wave" 1.0 true))))

(fn `Spawn Alien`
  ;[1 1 1] Spawn Alien at random valid target point
  (bind _spawn_point (`self.Get Random Spawn Point`))
  (`/Engine/EditorBlueprintResources/StandardMacros.IsValid` _spawn_point
    (:`Is Valid`
      (`|SpawnActorFromClass` "/Game/BluePrints/AI/BP_Alien.BP_Alien_C" (`self.GetTransform` _spawn_point) "Undefined" "OverrideRootScale" null null))))

(fn `UserConstructionScript`)